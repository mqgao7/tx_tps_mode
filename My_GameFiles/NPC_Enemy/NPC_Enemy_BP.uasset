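; Enemy NPC that carries a KA47 rifle, patrols random points in a fixed box and attacks the player.
; Pawn sensing speeds it up and starts a move toward the player plus a delayed firing loop that halts it and subtracts player health directly, without a trace.
; Its damage event tracks health; on death it awards the damage source a point, ragdolls with the gun, then destroys both.
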(event OnSeePawn(PawnSensing)
  (params (Pawn :type Pawn%20Object%20Reference))
  (if (not (Variables|Default|GetisDeath))
    (Variables|/Script/Engine.CharacterMovementComponent|SetMaxWalkSpeed (Variables|Character|GetCharacterMovement) 5e+02)
    (bind _asmy_character_bp (Utilities|Casting|CastToMy_Character_BP Pawn))
    (bind _output_get (Variables|Default|SetPlayer _asmy_character_bp))
    (AI|AIMoveTo self "0, 0, 0" _output_get 4e+02 false
      (:then
        (CallFunction|攻击玩家)))))

(event Custom|攻击玩家
  (bind _player (Variables|Default|GetPlayer))
  (bind _charactermovement (Variables|Character|GetCharacterMovement))
  (Utilities|FlowControl|Delay 4.0 :!label _label)
  (Variables|/Script/Engine.CharacterMovementComponent|SetMaxWalkSpeed _charactermovement 0.0)
  (Variables|/Script/Engine.CharacterMovementComponent|SetRotationRate _charactermovement "0, 0, 0")
  (Audio|PlaySound2D "/Game/My_Resource/Sound/sw_Wep_AR_Shoot_LP_End_01_Cue.sw_Wep_AR_Shoot_LP_End_01_Cue" 1.0 1.0 0.0 0 0)
  (Default|开火特效 (Variables|Default|GetKA47))
  (if (not (Variables|Default|GetisPlayerDeath))
    (Variables|/Game/My_GameFiles/Character/My_Character_BP.My_Character_BP_C|SetCurrentHealth _player (- (Variables|/Game/My_GameFiles/Character/My_Character_BP.My_Character_BP_C|GetCurrentHealth _player) 15.0))
    (Variables|Default|SetisPlayerDeath (<= (Variables|/Game/My_GameFiles/Character/My_Character_BP.My_Character_BP_C|GetCurrentHealth _player) 0.0))
    (goto _label)))

(event EventBeginPlay
  ;[1 1 1] 自动巡逻
  (bind _returnvalue (Game|SpawnActorfromClass "/Game/My_GameFiles/Weapon/KA47_CW_BP.KA47_CW_BP_C" (Transformation|GetSocketTransform (Variables|Character|GetMesh) "hand_r" "RTS_World") "Undefined" 0 0))
  (bind _output_get (Variables|Default|SetKA47 _returnvalue))
  (Transformation|AttachComponentToComponent _output_get (Variables|Character|GetMesh) "hand_r" "SnapToTarget" "SnapToTarget" "SnapToTarget" true)
  (Variables|/Script/Engine.CharacterMovementComponent|SetMaxWalkSpeed (Variables|Character|GetCharacterMovement) 1e+02)
  (AI|AIMoveTo self (Math|Random|RandomPointinBoundingBox "-1210.000000,2575.000000,144.000000" "1125.000000,870.000000,0.100000") 0 5.0 false :!label _label
    (:OnSuccess
      (Utilities|FlowControl|Delay 1.0)
      (goto _label))))

(event Event伤害传递
  (params (Damage :type Float%20%28single-precision%29) (伤害来源 :type My%20Character%20BP%20Object%20Reference))
  ;[1 1 1] 伤害传递和分数计算
  (Variables|Default|Set伤害来源 伤害来源)
  (bind _output_get (Variables|Default|SetCurrentHealth (- (Variables|Default|GetCurrentHealth) Damage)))
  (if (<= _output_get 0.0)
    (Variables|Default|SetisDeath true)
    (Utilities|FlowControl|DoOnce false
      (:Completed
        (bind _result (Math|Integer|IncrementInt (Variables|/Game/My_GameFiles/Character/My_Character_BP.My_Character_BP_C|Get得分 (Variables|Default|Get伤害来源)))
          (:%20%20
            (Variables|/Game/My_GameFiles/Character/My_Character_BP.My_Character_BP_C|Set得分 (Variables|Default|Get伤害来源) _result)
            (Components|Movement|StopMovementImmediately (Variables|Character|GetCharacterMovement))
            (Physics|SetSimulatePhysics (Variables|Character|GetMesh) true)
            (Physics|SetSimulatePhysics (Variables|/Game/My_GameFiles/Weapon/Weapon_BP.Weapon_BP_C|GetSkeletalMesh (Variables|Default|GetKA47)) true)
            (Utilities|FlowControl|Delay 1.0)
            (Actor|DestroyActor)
            (Actor|DestroyActor (Variables|Default|GetKA47))))))))

(fn ConstructionScript)