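; Weapon actor that the player character can pick up, carrying its stats, sounds and sockets in a WeaponInfo struct.
; Sphere overlap caches the character, enables input and calls its 捡起按下; leaving clears the pickup state.
; F or the weapon's own 捡起按下 event passes the weapon to the character's 捡取武器.
; The construction script writes the actor's class into WeaponInfo, and 开火特效 spawns muzzle flash at the Arrow.
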(event OnComponentBeginOverlap(Sphere)
  (params (OverlappedComponent :type Primitive%20Component%20Object%20Reference) (OtherActor :type Actor%20Object%20Reference) (OtherComp :type Primitive%20Component%20Object%20Reference) (OtherBodyIndex :type Integer) (bFromSweep :type Boolean) (SweepResult :type Hit%20Result%20Structure%20%28by%20ref%29))
  (bind _asmy_character_bp (Utilities|Casting|CastToMy_Character_BP OtherActor))
  (bind _output_get (Variables|Default|SetAs%20My%20Character%20BP _asmy_character_bp))
  (Variables|Default|SetCanPickUp true)
  (Input|EnableInput (Game|GetPlayerController 0))
  (Default|捡起按下 _output_get self))

(event OnComponentEndOverlap(Sphere)
  (params (OverlappedComponent :type Primitive%20Component%20Object%20Reference) (OtherActor :type Actor%20Object%20Reference) (OtherComp :type Primitive%20Component%20Object%20Reference) (OtherBodyIndex :type Integer))
  (Variables|Default|SetAs%20My%20Character%20BP 0)
  (Variables|Default|SetCanPickUp false))

(event Custom|开火特效
  (bind _arrow (Variables|Default|GetArrow))
  (bind _returnvalue (Transformation|GetWorldTransform _arrow))
  (Effects|SpawnEmitteratLocation "/Game/My_Resource/FX/P_AssaultRifle_MuzzleFlash.P_AssaultRifle_MuzzleFlash" (.location _returnvalue) (.rotation _returnvalue)))

(event Custom|捡起按下
  (bind _as_my_character_bp (Variables|Default|GetAs%20My%20Character%20BP))
  (Utilities|IsValid _as_my_character_bp
    (:Is%20Valid
      (if (Variables|Default|GetCanPickUp)
        (Default|捡取武器 _as_my_character_bp self)))))

(event Input|KeyboardEvents|F
  (params (Key :type Key%20Structure :default "None"))
  (bind _as_my_character_bp (Variables|Default|GetAs%20My%20Character%20BP))
  (:Pressed
    (Utilities|IsValid _as_my_character_bp
      (:Is%20Valid
        (if (Variables|Default|GetCanPickUp)
          (Default|捡取武器 _as_my_character_bp self))))))

(fn ConstructionScript
  (Variables|Default|SetWeaponInfo (Utilities|Struct|MakeWeaponInfo (.weapontype (Variables|Default|GetWeaponInfo)) (.weaponname (Variables|Default|GetWeaponInfo)) (Utilities|GetClass self) (.weaponicon (Variables|Default|GetWeaponInfo)) (.shootingspeed (Variables|Default|GetWeaponInfo)) (.shootingsound (Variables|Default|GetWeaponInfo)) (.curcapacity (Variables|Default|GetWeaponInfo)) (.maxcapacity (Variables|Default|GetWeaponInfo)) (.maxammo (Variables|Default|GetWeaponInfo)) (.weapondamage (Variables|Default|GetWeaponInfo)) (.weaponequipsocket (Variables|Default|GetWeaponInfo)) (.weaponholdsocket (Variables|Default|GetWeaponInfo)) (.捡起声音 (Variables|Default|GetWeaponInfo)) (.装备声音 (Variables|Default|GetWeaponInfo)) (.射击距离 (Variables|Default|GetWeaponInfo)) (.射击montage (Variables|Default|GetWeaponInfo)) (.武器子弹耗尽声音 (Variables|Default|GetWeaponInfo)))))