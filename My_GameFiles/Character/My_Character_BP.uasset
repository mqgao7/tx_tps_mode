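; Third-person shooter player character with keyboard and touch movement, sprint, scope zoom, grenade throws, and ragdoll game-over on death.
; Picked-up weapons attach to mesh sockets tracked in a map, supporting montage-based equip, holster and cycling.
; Firing loops camera line traces on a timer, applying damage through Damage_Interface.
; Custom events mirror most input actions, and 行动模式 switches between controller-yaw and movement-facing rotation.
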(event EventBeginPlay)

(event Collision|EventActorBeginOverlap
  (params (OtherActor :type Actor%20Object%20Reference)))

(event EventTick
  (params (DeltaSeconds :type Float%20%28single-precision%29)))

(event Custom|Jump%20Stop
  ;[1 1 1] 基础移动
  (Character|StopJumping))

(event Custom|Jump%20Start
  ;[1 1 1] 基础移动
  (Character|Jump))

(event Custom|Input%20touch
  ;[1 1 1] 触控旋转视角
  (Utilities|FlowControl|Gate true
    (:Exit
      (if (>= (Math|Vector2D|Vector2DLength (- (Math|Vector2D|MakeVector2D (.LocationX (Class|PlayerController|GetInputTouchState (Game|GetPlayerController 0) (stale Input|TouchEvents|InputTouch FingerIndex))) (.LocationY (Class|PlayerController|GetInputTouchState (Game|GetPlayerController 0) (stale Input|TouchEvents|InputTouch FingerIndex)))) (Variables|Default|GetTouch%20Vector2))) (Variables|Default|GetNewVar_0))
        (Variables|Default|SetTouch%20Vector1 "(X=100000.000000,Y=1000000.000000)")
        (Pawn|Input|AddControllerYawInput (.x (* (- (Math|Vector2D|MakeVector2D (.LocationX (Class|PlayerController|GetInputTouchState (Game|GetPlayerController 0) (stale Input|TouchEvents|InputTouch FingerIndex))) (.LocationY (Class|PlayerController|GetInputTouchState (Game|GetPlayerController 0) (stale Input|TouchEvents|InputTouch FingerIndex)))) (Variables|Default|GetTouch%20Vector2)) (Variables|Default|GetNewVar_0))))
        (Pawn|Input|AddControllerPitchInput (.y (* (- (Math|Vector2D|MakeVector2D (.LocationX (Class|PlayerController|GetInputTouchState (Game|GetPlayerController 0) (stale Input|TouchEvents|InputTouch FingerIndex))) (.LocationY (Class|PlayerController|GetInputTouchState (Game|GetPlayerController 0) (stale Input|TouchEvents|InputTouch FingerIndex)))) (Variables|Default|GetTouch%20Vector2)) (Variables|Default|GetNewVar_0))))))))

(event Custom|冲刺按下
  ;[1 1 1] 冲刺
  (if (not (Variables|Default|GetisOpenScope))
    (Variables|Default|SetisSpring true)
    (CallFunction|行动模式 false true)
    (bind _新建轨道_0 (Timeline|时间轴_1 Play)
      (:Update
        (Variables|/Script/Engine.CharacterMovementComponent|SetMaxWalkSpeed (Variables|Character|GetCharacterMovement) (Math|Float|Lerp 4e+02 6e+02 _新建轨道_0))))))

(event Custom|冲刺松开
  ;[1 1 1] 冲刺
  (if (not (Variables|Default|GetisOpenScope))
    (Variables|Default|SetisSpring false)
    (CallFunction|行动模式 true false)
    (bind _新建轨道_0 (Timeline|时间轴_1 Reverse)
      (:Update
        (Variables|/Script/Engine.CharacterMovementComponent|SetMaxWalkSpeed (Variables|Character|GetCharacterMovement) (Math|Float|Lerp 4e+02 6e+02 _新建轨道_0))))))

(event Input|ActionEvents|InputActionJump
  (params (Key :type Key%20Structure :default "None"))
  ;[1 1 1] 基础移动
  (:Pressed
    (Character|Jump))
  (:Released
    (Character|StopJumping)))

(event Input|ActionEvents|InputActionSpring
  (params (Key :type Key%20Structure :default "None"))
  (bind _isopenscope (Variables|Default|GetisOpenScope))
  (bind _returnvalue (not _isopenscope))
  ;[1 1 1] 冲刺
  (:Pressed
    (if _returnvalue
      (Variables|Default|SetisSpring true)
      (CallFunction|行动模式 false true)
      (bind _新建轨道_0 (Timeline|时间轴_1 Play)
        (:Update
          (Variables|/Script/Engine.CharacterMovementComponent|SetMaxWalkSpeed (Variables|Character|GetCharacterMovement) (Math|Float|Lerp 4e+02 6e+02 _新建轨道_0))))))
  (:Released
    (if _returnvalue
      (Variables|Default|SetisSpring false)
      (CallFunction|行动模式 true false)
      (Timeline|时间轴_1 Reverse))))

(event Input|AxisEvents|InputAxisMoveForward
  (params (AxisValue :type Float%20%28single-precision%29))
  ;[1 1 1] 基础移动
  (Pawn|Input|AddMovementInput (Math|Vector|GetForwardVector (Pawn|GetControlRotation :!class /Script/Engine.Pawn)) AxisValue false))

(event Input|AxisEvents|InputAxisMoveRight
  (params (AxisValue :type Float%20%28single-precision%29))
  ;[1 1 1] 基础移动
  (Pawn|Input|AddMovementInput (Math|Vector|GetRightVector (Pawn|GetControlRotation :!class /Script/Engine.Pawn)) AxisValue false))

(event Input|AxisEvents|InputAxisTurn
  (params (AxisValue :type Float%20%28single-precision%29))
  ;[1 1 1] 基础移动
  (Pawn|Input|AddControllerYawInput AxisValue))

(event Input|AxisEvents|InputAxisLookUp
  (params (AxisValue :type Float%20%28single-precision%29))
  ;[1 1 1] 基础移动
  (Pawn|Input|AddControllerPitchInput AxisValue))

(event Input|TouchEvents|InputTouch
  (params (Location :type Vector) (FingerIndex :type ETouchIndex%20Enum))
  (bind _returnvalue (Game|GetPlayerController 0))
  (bind (_locationx _locationy) (Class|PlayerController|GetInputTouchState _returnvalue FingerIndex))
  (bind _returnvalue_2 (Math|Vector2D|MakeVector2D _locationx _locationy))
  ;[1 1 1] 触控旋转视角
  (:Pressed
    (bind _output_get (Variables|Default|SetTouch%20Vector1 _returnvalue_2))
    (Variables|Default|SetTouch%20Vector2 _output_get)
    (Utilities|FlowControl|Gate true) ; enters at Open
  )
  (:Released
    (Utilities|FlowControl|Gate true) ; enters at Close
  ))

(event Custom|get%20server
  (params (server :type Blueprint%20Session%20Result%20Structure))
  (Development|PrintString (Utilities|String|ToString(Integer) (Class|FindSessionsCallbackProxy|GetCurrentPlayers server))))

(event Custom|拔枪
  ;[1 1 1] 收枪拔枪
  (Variables|Default|SetwithWeapon true)
  (Development|PrintString "装备武器")
  (Animation|PlayAnimMontage "/Game/AnimStarterPack/Equip_Rifle_Standing_Montage.Equip_Rifle_Standing_Montage" 2.0 "None")
  (CallFunction|行动模式 true false))

(event Custom|开火按下
  (bind _currentweapon (Variables|Default|GetCurrentWeapon))
  (bind _weaponinfo (Variables|/Game/My_GameFiles/Weapon/Weapon_BP.Weapon_BP_C|GetWeaponInfo _currentweapon))
  (bind (_shootingspeed _curcapacity) (Utilities|Struct|BreakWeaponInfo _weaponinfo))
  ;[1 1 1] 武器开火
  (if (and (Variables|Default|GetwithWeapon) (not (Variables|Default|GetisSpring)))
    (CallFunction|Shooting)
    (if (== _curcapacity 0)
      (Utilities|Time|ClearandInvalidateTimerbyHandle (Variables|Default|GetTimerHandle))
      (else
        (bind _returnvalue (Utilities|Time|SetTimerbyEvent (delegate Custom|Shooting) _shootingspeed true))
        (Variables|Default|SetTimerHandle _returnvalue)))))

(event Custom|切换按下
  (bind _socketweaponstate (Variables|Default|GetSocketWeaponState))
  ;[1 1 1] Q切换武器
  (if (Variables|Default|GetwithWeapon)
    (if (> (Utilities|Map|Length _socketweaponstate) 1)
      (bind _values (Utilities|Map|Values _socketweaponstate))
      (Variables|Default|SetWeaponsArrayCache _values)
      (bind _output_get (Variables|Default|SetCurrentNextWeaponIndex (+ (Utilities|Array|FindItem (Variables|Default|GetWeaponsArrayCache) (Variables|Default|GetCurrentWeapon)) 1)))
      (if (Utilities|Array|IsValidIndex (Variables|Default|GetWeaponsArrayCache) _output_get)
        (CallFunction|收枪)
        (Utilities|FlowControl|Delay 0.6)
        (Variables|Default|SetCurrentWeapon (Utilities|Array|Get(acopy) (Variables|Default|GetWeaponsArrayCache) (Variables|Default|GetCurrentNextWeaponIndex)))
        (CallFunction|拔枪)
        (else
          (CallFunction|收枪)
          (Utilities|FlowControl|Delay 0.6)
          (Variables|Default|SetCurrentWeapon (Utilities|Array|Get(acopy) (Variables|Default|GetWeaponsArrayCache)))
          (CallFunction|拔枪))))))

(event Custom|卸载按下
  ;[1 1 1] 收枪拔枪
  (Utilities|IsValid (Variables|Default|GetCurrentWeapon)
    (:Is%20Valid
      (if (Variables|Default|GetwithWeapon)
        (Variables|Default|SetwithWeapon false)
        (Development|PrintString "卸载武器")
        (Animation|PlayAnimMontage "/Game/AnimStarterPack/Unequip_Rifle_Standing_Montage.Unequip_Rifle_Standing_Montage" 2.0 "None")
        (CallFunction|行动模式 false true)
        (else
          (Variables|Default|SetwithWeapon true)
          (Development|PrintString "装备武器")
          (Animation|PlayAnimMontage "/Game/AnimStarterPack/Equip_Rifle_Standing_Montage.Equip_Rifle_Standing_Montage" 2.0 "None")
          (CallFunction|行动模式 true false))))
    (:Is%20Not%20Valid
      (Development|PrintString "尚未装备武器"))))

(event Custom|手雷按下
  (if (Variables|Default|GetwithWeapon)
    (CallFunction|收枪)
    (Utilities|FlowControl|Delay 1.0))
  (bind _returnvalue (Game|SpawnActorfromClass "/Game/My_GameFiles/Weapon/Grenade_BP.Grenade_BP_C" (Transformation|GetSocketTransform (Variables|Character|GetMesh) "hand_r_Gre" "RTS_World") "Undefined" 0 0))
  (bind _output_get (Variables|Default|SetGrenade _returnvalue))
  (Transformation|AttachComponentToComponent _output_get (Variables|Character|GetMesh) "hand_r_Gre" "SnapToTarget" "SnapToTarget" "SnapToTarget" true)
  (Animation|PlayAnimMontage "/Game/My_GameFiles/Character/ThrowSingle1_Montage.ThrowSingle1_Montage" 1.0 "None"))

(event Custom|收枪
  ;[1 1 1] 收枪拔枪
  (Variables|Default|SetwithWeapon false)
  (Development|PrintString "卸载武器")
  (Animation|PlayAnimMontage "/Game/AnimStarterPack/Unequip_Rifle_Standing_Montage.Unequip_Rifle_Standing_Montage" 2.0 "None")
  (CallFunction|行动模式 false true))

(event Custom|挂载武器
  (bind _currentweapon (Variables|Default|GetCurrentWeapon))
  (bind _weaponinfo (Variables|/Game/My_GameFiles/Weapon/Weapon_BP.Weapon_BP_C|GetWeaponInfo _currentweapon))
  (bind (_weapondamage _weaponequipsocket _weaponholdsocket _捡起声音 _装备声音) (Utilities|Struct|BreakWeaponInfo _weaponinfo))
  ;[1 1 1] 收枪拔枪
  (Transformation|AttachComponentToComponent _currentweapon (Variables|Character|GetMesh) _weaponequipsocket "SnapToTarget" "SnapToTarget" "SnapToTarget" true)
  (Audio|PlaySound2D _捡起声音 1.0 1.0 0.0 0 0))

(event Custom|装备武器
  (bind _currentweapon (Variables|Default|GetCurrentWeapon))
  (bind _weaponinfo (Variables|/Game/My_GameFiles/Weapon/Weapon_BP.Weapon_BP_C|GetWeaponInfo _currentweapon))
  (bind (_weapondamage _weaponequipsocket _weaponholdsocket _捡起声音 _装备声音) (Utilities|Struct|BreakWeaponInfo _weaponinfo))
  ;[1 1 1] 收枪拔枪
  (Transformation|AttachComponentToComponent _currentweapon (Variables|Character|GetMesh) _weaponholdsocket "SnapToTarget" "SnapToTarget" "SnapToTarget" true)
  (Audio|PlaySound2D _装备声音 1.0 1.0 0.0 0 0))

(event Custom|Shooting
  (bind _camera (Variables|Default|GetCamera))
  (bind _currentweapon (Variables|Default|GetCurrentWeapon))
  (bind _currentweapon_2 (Variables|Default|GetCurrentWeapon))
  (bind _currentweapon_3 (Variables|Default|GetCurrentWeapon))
  (bind _returnvalue (Transformation|GetWorldLocation _camera))
  (bind _weaponinfo (Variables|/Game/My_GameFiles/Weapon/Weapon_BP.Weapon_BP_C|GetWeaponInfo _currentweapon))
  (bind _weaponinfo_2 (Variables|/Game/My_GameFiles/Weapon/Weapon_BP.Weapon_BP_C|GetWeaponInfo _currentweapon_2))
  (bind (_curcapacity _weapondamage) (Utilities|Struct|BreakWeaponInfo _weaponinfo))
  (bind (_shootingsound _射击montage _武器子弹耗尽声音) (Utilities|Struct|BreakWeaponInfo _weaponinfo_2))
  ;[1 1 1] 武器开火
  (if (== (.CurCapacity (Utilities|Struct|BreakWeaponInfo (Variables|/Game/My_GameFiles/Weapon/Weapon_BP.Weapon_BP_C|GetWeaponInfo (Variables|Default|GetCurrentWeapon)))) 0)
    (Development|PrintString "缺少弹药")
    (Audio|PlaySound2D _武器子弹耗尽声音 1.0 1.0 0.0 0 0)
    (Utilities|Time|ClearandInvalidateTimerbyHandle (Variables|Default|GetTimerHandle))
    (else
      (Animation|PlayAnimMontage _射击montage 1.0 "None")
      (Audio|PlaySound2D _shootingsound 1.0 1.0 0.0 0 0)
      (Default|开火特效 _currentweapon_3)
      (bind _outhit (Collision|LineTraceByChannel _returnvalue (+ _returnvalue (* (Math|Vector|GetForwardVector _camera) (Utilities|Struct|BreakWeaponInfo (Variables|/Game/My_GameFiles/Weapon/Weapon_BP.Weapon_BP_C|GetWeaponInfo (Variables|Default|GetCurrentWeapon))))) "TraceTypeQuery1" false (Utilities|Array|MakeArray _currentweapon_3) "ForDuration"))
      (Math|Integer|DecrementInt _curcapacity
        (:%20%20
          (Development|PrintString (Utilities|GetDisplayName (.HitActor (Collision|BreakHitResult _outhit))))
          (if (Utilities|DoesObjectImplementInterface (.HitActor (Collision|BreakHitResult _outhit)) "/Game/My_GameFiles/Interface/Damage_Interface.Damage_Interface_C")
            (Class|DamageInterface|伤害传递(Message) (.HitActor (Collision|BreakHitResult _outhit)) _weapondamage self)))))))

(event Custom|捡起按下
  (params (NewParam :type Weapon%20BP%20Object%20Reference))
  ;[1 1 1] 捡起武器
  (Variables|Default|Set重叠武器 NewParam))

(event Custom|扔手雷
  (Transformation|DetachFromActor (Variables|Default|GetGrenade) "KeepWorld" "KeepWorld" "KeepWorld")
  (Physics|SetSimulatePhysics (Variables|/Game/My_GameFiles/Weapon/Grenade_BP.Grenade_BP_C|GetStaticMesh (Variables|Default|GetGrenade)) true)
  (Physics|SetPhysicsLinearVelocity (Variables|/Game/My_GameFiles/Weapon/Grenade_BP.Grenade_BP_C|GetStaticMesh (Variables|Default|GetGrenade)) (* (Math|Vector|GetForwardVector (Transformation|GetActorRotation)) 1e+03) false "None"))

(event Custom|捡取武器
  (params (Weapon :type Weapon%20BP%20Object%20Reference))
  ;[1 1 1] 捡起武器
  (Variables|Default|SetWeapon Weapon)
  (if (Variables|Default|GetwithWeapon)
    (if (Utilities|IsValid (.Value (Utilities|Map|Find (Variables|Default|GetSocketWeaponState) (.WeaponEquipSocket (Utilities|Struct|BreakWeaponInfo (Variables|/Game/My_GameFiles/Weapon/Weapon_BP.Weapon_BP_C|GetWeaponInfo (Variables|Default|GetWeapon)))))))
      (Development|PrintString "插槽被占用")
      (else
        (Transformation|AttachComponentToComponent (Variables|Default|GetWeapon) (Variables|Character|GetMesh) (.WeaponEquipSocket (Utilities|Struct|BreakWeaponInfo (Variables|/Game/My_GameFiles/Weapon/Weapon_BP.Weapon_BP_C|GetWeaponInfo (Variables|Default|GetWeapon)))) "SnapToTarget" "SnapToTarget" "SnapToTarget" true)
        (Utilities|Map|Add (Variables|Default|GetSocketWeaponState) (.WeaponEquipSocket (Utilities|Struct|BreakWeaponInfo (Variables|/Game/My_GameFiles/Weapon/Weapon_BP.Weapon_BP_C|GetWeaponInfo (Variables|Default|GetWeapon)))) (Variables|Default|GetWeapon))
        (Audio|PlaySound2D (.捡起声音 (Utilities|Struct|BreakWeaponInfo (Variables|/Game/My_GameFiles/Weapon/Weapon_BP.Weapon_BP_C|GetWeaponInfo (Variables|Default|GetWeapon)))) 1.0 1.0 0.0 0 0)))
    (elif (Utilities|IsValid (.Value (Utilities|Map|Find (Variables|Default|GetSocketWeaponState) (.WeaponEquipSocket (Utilities|Struct|BreakWeaponInfo (Variables|/Game/My_GameFiles/Weapon/Weapon_BP.Weapon_BP_C|GetWeaponInfo (Variables|Default|GetWeapon)))))))
      (Development|PrintString "插槽被占用")
      (else
        (bind _output_get (Variables|Default|SetCurrentWeapon (Variables|Default|GetWeapon)))
        (Transformation|AttachComponentToComponent _output_get (Variables|Character|GetMesh) (.WeaponHoldSocket (Utilities|Struct|BreakWeaponInfo (Variables|/Game/My_GameFiles/Weapon/Weapon_BP.Weapon_BP_C|GetWeaponInfo _output_get))) "SnapToTarget" "SnapToTarget" "SnapToTarget" true)
        (Utilities|Map|Add (Variables|Default|GetSocketWeaponState) (.WeaponEquipSocket (Utilities|Struct|BreakWeaponInfo (Variables|/Game/My_GameFiles/Weapon/Weapon_BP.Weapon_BP_C|GetWeaponInfo _output_get))) _output_get)
        (Audio|PlaySound2D (.装备声音 (Utilities|Struct|BreakWeaponInfo (Variables|/Game/My_GameFiles/Weapon/Weapon_BP.Weapon_BP_C|GetWeaponInfo _output_get))) 1.0 1.0 0.0 0 0)
        (Variables|Default|SetwithWeapon true)
        (CallFunction|行动模式 true false)))))

(event Custom|开火松开
  (bind _timerhandle (Variables|Default|GetTimerHandle))
  ;[1 1 1] 武器开火
  (if (Utilities|Time|IsValidTimerHandle _timerhandle)
    (Utilities|Time|ClearandInvalidateTimerbyHandle _timerhandle)))

(event EventTick
  (params (DeltaSeconds :type Float%20%28single-precision%29))
  (bind _returnvalue (Game|GetPlayerController 0))
  (CallFunction|InputTouch)
  (if (<= (Variables|Default|GetCurrentHealth) 0.0)
    (Components|Movement|StopMovementImmediately (Variables|Character|GetCharacterMovement))
    (Physics|SetSimulatePhysics (Variables|Character|GetMesh) true)
    (Utilities|FlowControl|Delay 2.0)
    (bind _returnvalue_2 (UserInterface|CreateWidget "/Game/My_GameFiles/Game_UI/GameOver_UI.GameOver_UI_C"))
    (UserInterface|Viewport|AddtoViewport _returnvalue_2 0)
    (Variables|/Script/Engine.PlayerController|SetbShowMouseCursor _returnvalue true)
    (Input|SetInputModeUIOnly _returnvalue 0 "DoNotLock")
    (Game|SetGamePaused true)))

(event EventBeginPlay
  (bind _returnvalue (Game|GetCurrentLevelName true))
  (if (Utilities|Enum|Equal(Enum) _returnvalue "ThirdPersonExampleMap")
    (Class|PlayerController|ActivateTouchInterface (Game|GetPlayerController (Class|FindSessionsCallbackProxy|GetCurrentPlayers (stale Custom|get%20server server))) "/Game/My_GameFiles/Game_UI/MyVirtualJoysticks.MyVirtualJoysticks")
    (bind _returnvalue_2 (UserInterface|CreateWidget "/Game/My_GameFiles/Game_UI/MainWidget_UI.MainWidget_UI_C" (Game|GetPlayerController (Class|FindSessionsCallbackProxy|GetCurrentPlayers (stale Custom|get%20server server)))))
    (bind _output_get (Variables|Default|SetMainUI _returnvalue_2))
    (UserInterface|Viewport|AddtoViewport _output_get 0)
    (Variables|Default|SetMaxHealth (Variables|Default|GetMaxHealth))))

(event Input|ActionEvents|InputActionEquip/UnEquip
  (params (Key :type Key%20Structure :default "None"))
  ;[1 1 1] 收枪拔枪
  (:Pressed
    (Utilities|IsValid (Variables|Default|GetCurrentWeapon)
      (:Is%20Valid
        (if (Variables|Default|GetwithWeapon)
          (Variables|Default|SetwithWeapon false)
          (Development|PrintString "卸载武器")
          (Animation|PlayAnimMontage "/Game/AnimStarterPack/Unequip_Rifle_Standing_Montage.Unequip_Rifle_Standing_Montage" 2.0 "None")
          (CallFunction|行动模式 false true)
          (else
            (Variables|Default|SetwithWeapon true)
            (Development|PrintString "装备武器")
            (Animation|PlayAnimMontage "/Game/AnimStarterPack/Equip_Rifle_Standing_Montage.Equip_Rifle_Standing_Montage" 2.0 "None")
            (CallFunction|行动模式 true false))))
      (:Is%20Not%20Valid
        (Development|PrintString "尚未装备武器")))))

(event Input|ActionEvents|InputActionSwitchWeapon
  (params (Key :type Key%20Structure :default "None"))
  (bind _socketweaponstate (Variables|Default|GetSocketWeaponState))
  ;[1 1 1] Q切换武器
  (:Pressed
    (if (Variables|Default|GetwithWeapon)
      (if (> (Utilities|Map|Length _socketweaponstate) 1)
        (bind _values (Utilities|Map|Values _socketweaponstate))
        (Variables|Default|SetWeaponsArrayCache _values)
        (bind _output_get (Variables|Default|SetCurrentNextWeaponIndex (+ (Utilities|Array|FindItem (Variables|Default|GetWeaponsArrayCache) (Variables|Default|GetCurrentWeapon)) 1)))
        (if (Utilities|Array|IsValidIndex (Variables|Default|GetWeaponsArrayCache) _output_get)
          (CallFunction|收枪)
          (Utilities|FlowControl|Delay 0.6)
          (Variables|Default|SetCurrentWeapon (Utilities|Array|Get(acopy) (Variables|Default|GetWeaponsArrayCache) (Variables|Default|GetCurrentNextWeaponIndex)))
          (CallFunction|拔枪)
          (else
            (CallFunction|收枪)
            (Utilities|FlowControl|Delay 0.6)
            (Variables|Default|SetCurrentWeapon (Utilities|Array|Get(acopy) (Variables|Default|GetWeaponsArrayCache)))
            (CallFunction|拔枪)))))))

(event Input|ActionEvents|InputActionThrow
  (params (Key :type Key%20Structure :default "None"))
  (:Pressed
    (if (Variables|Default|GetwithWeapon)
      (CallFunction|收枪)
      (Utilities|FlowControl|Delay 1.0))
    (bind _returnvalue (Game|SpawnActorfromClass "/Game/My_GameFiles/Weapon/Grenade_BP.Grenade_BP_C" (Transformation|GetSocketTransform (Variables|Character|GetMesh) "hand_r_Gre" "RTS_World") "Undefined" 0 0))
    (bind _output_get (Variables|Default|SetGrenade _returnvalue))
    (Transformation|AttachComponentToComponent _output_get (Variables|Character|GetMesh) "hand_r_Gre" "SnapToTarget" "SnapToTarget" "SnapToTarget" true)
    (Animation|PlayAnimMontage "/Game/My_GameFiles/Character/ThrowSingle1_Montage.ThrowSingle1_Montage" 1.0 "None")))

(event Input|ActionEvents|InputActionFireWeapon
  (params (Key :type Key%20Structure :default "None"))
  (bind _currentweapon (Variables|Default|GetCurrentWeapon))
  (bind _weaponinfo (Variables|/Game/My_GameFiles/Weapon/Weapon_BP.Weapon_BP_C|GetWeaponInfo _currentweapon))
  (bind (_shootingspeed _curcapacity) (Utilities|Struct|BreakWeaponInfo _weaponinfo))
  ;[1 1 1] 武器开火
  (:Pressed
    (if (and (Variables|Default|GetwithWeapon) (not (Variables|Default|GetisSpring)))
      (CallFunction|Shooting)
      (if (== _curcapacity 0)
        (Utilities|Time|ClearandInvalidateTimerbyHandle (Variables|Default|GetTimerHandle) :!label _label)
        (else
          (bind _returnvalue (Utilities|Time|SetTimerbyEvent (delegate Custom|Shooting) _shootingspeed true))
          (Variables|Default|SetTimerHandle _returnvalue)))))
  (:Released
    (if (Utilities|Time|IsValidTimerHandle (Variables|Default|GetTimerHandle))
      (goto _label))))

(event Input|ActionEvents|InputActionOpenScope
  (params (Key :type Key%20Structure :default "None"))
  ;[1 1 1] 镜头拉伸
  (:Pressed
    (if (and (Variables|Default|GetwithWeapon) (not (Variables|Default|GetisSpring)))
      (Utilities|FlowControl|FlipFlop
        (:A
          (Variables|Default|SetisOpenScope true)
          (bind _新建轨道_0 (Timeline|时间轴_0 Play)
            (:Update
              (Variables|/Script/Engine.SpringArmComponent|SetTargetArmLength (Variables|Default|GetSpringArm) (Math|Float|Lerp 3e+02 8e+01 _新建轨道_0)))))
        (:B
          (Variables|Default|SetisOpenScope false)
          (Timeline|时间轴_0 Reverse))))))

(fn ConstructionScript)

(fn 行动模式
  (params (使用控制器旋转Yaw :type Boolean) (将旋转朝向运动 :type Boolean))
  (Variables|Default|SetbUseControllerRotationYaw 使用控制器旋转Yaw)
  (Variables|/Script/Engine.CharacterMovementComponent|SetbOrientRotationToMovement (Variables|Character|GetCharacterMovement) 将旋转朝向运动))