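; Target actor that takes damage and awards a point to whoever destroys it.
; The 伤害传递 (damage transfer) event stores the damage source and subtracts the damage from CurrentHealth.
; At zero health it flags death and, guarded by a DoOnce, increments the source's 得分 (score), turns on physics for Cube and Cylinder1, then destroys itself after a short delay.
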(event Event伤害传递
  (params (Damage :type Float%20%28single-precision%29) (伤害来源 :type My%20Character%20BP%20Object%20Reference))
  (Variables|Default|Set伤害来源 伤害来源)
  (bind _output_get (Variables|Default|SetCurrentHealth (- (Variables|Default|GetCurrentHealth) Damage)))
  (if (<= _output_get 0.0)
    (Variables|Default|SetisDeath true)
    (Utilities|FlowControl|DoOnce false
      (:Completed
        (bind _result (Math|Integer|IncrementInt (Variables|/Game/My_GameFiles/Character/My_Character_BP.My_Character_BP_C|Get得分 (Variables|Default|Get伤害来源)))
          (:%20%20
            (Variables|/Game/My_GameFiles/Character/My_Character_BP.My_Character_BP_C|Set得分 (Variables|Default|Get伤害来源) _result)
            (Physics|SetSimulatePhysics (Variables|Default|GetCube) true)
            (Utilities|FlowControl|Delay 3.0)
            (Actor|DestroyActor)))))))

(fn ConstructionScript)